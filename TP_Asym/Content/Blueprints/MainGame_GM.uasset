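; Game mode that lets the player start as either a turret pawn or a first-person pawn.
; On BeginPlay it creates the Selection_HUD widget and adds it to the viewport.
; StartAsTurret and StartAsFirstPerson each find the matching pawn already placed in the level, store the reference, and have player controller 0 possess it.
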(event `self.ReceiveBeginPlay`
  (bind _returnvalue (`|CreateWidget` "/Game/Widgets/Selection_HUD.Selection_HUD_C"))
  (`UserWidget.AddToViewport` _returnvalue 0))

(fn `StartAsFirstPerson`
  (bind _returnvalue (`GameplayStatics.GetPlayerController` 0))
  ;[0.2517 0.5163 1] Récupère la référence du joueur et set la variable Turret
  (bind _returnvalue_2 (`GameplayStatics.GetActorOfClass` "/Game/Pawns/BP_Pawn_FirstPerson.BP_Pawn_FirstPerson_C"))
  (set `self.FirstPerson` _returnvalue_2)
  ;[0.9234 0.1284 1] Set le joueur au pawn correspondant
  (cast `PlayerController` _returnvalue)
  (`Controller.Possess` _returnvalue (`self.FirstPerson`)))

(fn `StartAsTurret`
  (bind _returnvalue (`GameplayStatics.GetPlayerController` 0))
  ;[0.2517 0.5163 1] Récupère la référence du joueur et set la variable Turret
  (bind _returnvalue_2 (`GameplayStatics.GetActorOfClass` "/Game/Pawns/BP_Pawn_Turret.BP_Pawn_Turret_C"))
  (set `self.Turret` _returnvalue_2)
  ;[0.9234 0.1284 1] Set le joueur au pawn correspondant
  (cast `PlayerController` _returnvalue)
  (`Controller.Possess` _returnvalue (`self.Turret`)))

(fn `UserConstructionScript`)