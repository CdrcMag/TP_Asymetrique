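; Menu_PC is the main menu player controller that shows the menu HUD and starts or joins a multiplayer game.
; On begin play it adds the Menu_HUD widget to the viewport and shows the mouse cursor in game-and-UI input mode.
; Host creates a two-connection online session, then opens MainMap as a listen server.
; Join connects by running an "open" console command built from the supplied address string.
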(event `self.ReceiveBeginPlay`
  (`self.HUD_Menu`)
  (`self.Init_Mouse`))

(event `Init_Mouse`
  (set `self.bShowMouseCursor` true)
  (`WidgetBlueprintLibrary.SetInputMode_GameAndUIEx` self null "LockAlways" false))

(event `HUD_Menu`
  (bind _returnvalue (`|CreateWidget` "/Game/Widgets/Menu_HUD.Menu_HUD_C" self))
  (`UserWidget.AddToViewport` _returnvalue 0))

(event `Host`
  (`CreateSessionCallbackProxy.CreateSession` self 2
    (:`OnSuccess`
      (`GameplayStatics.OpenLevel` "MainMap" true "listen"))))

(event `Join`
  (params (B :type String))
  (`KismetSystemLibrary.ExecuteConsoleCommand` (`KismetStringLibrary.Concat_StrStr` "open " B) null))

(fn `UserConstructionScript`)